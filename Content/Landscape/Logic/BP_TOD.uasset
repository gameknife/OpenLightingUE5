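; Time-of-day controller that drives the sun, sky sphere, sky light, fog and global illumination from a single TimeOfDay value.
; Tick eases TimeOfDay toward TargetTimeOfDay, which optionally auto-advances, while the construction script creates the sky material instance and applies the current time.
; SetTimeOfDay samples curves for sun pitch, intensity, temperature, illumination and fog.
; A curve-derived sun height picks sky, cloud, fog and skylight colors and blends in stars below zero.
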(event `self.ReceiveTick`
  (params (DeltaSeconds :type "Float (single-precision)"))
  (if (`self.AutoPlay`)
    (set `self.TargetTimeOfDay` (+ (`self.TargetTimeOfDay`) (* DeltaSeconds (`self.AutoPlaySpeed`)))))
  (`self.SetTimeOfDay` (`KismetMathLibrary.Lerp` (`self.TimeOfDay`) (`self.TargetTimeOfDay`) 0.1)))

(fn `RefreshMaterial`
  (bind _sky_material (`self.Sky material`))
  (bind _sun_height (`self.Sun height`))
  (bind _sky_material_2 (`self.Sky material`))
  (bind _sky_material_3 (`self.Sky material`))
  (bind _returnvalue (`CurveLinearColor.GetClampedLinearColorValue` (`self.Horizon color curve`) (`self.Sun height`)))
  (`/Engine/EditorBlueprintResources/StandardMacros.IsValid` (`self.Directional light actor`) ; Has a directional light been assigned?
    (:`Is Valid`
      (`MaterialInstanceDynamic.SetVectorParameterValue` _sky_material "Light direction" (`KismetMathLibrary.Conv_VectorToLinearColor` (`KismetMathLibrary.Conv_RotatorToVector` (`self.K2_GetActorRotation` (`self.Directional light actor`)))))
      (`MaterialInstanceDynamic.SetVectorParameterValue` _sky_material "Sun color" (`KismetMathLibrary.Conv_ColorToLinearColor` (`LightComponentBase.LightColor` (`Light.LightComponent` (`self.Directional light actor`)))))
      (`MaterialInstanceDynamic.SetVectorParameterValue` _sky_material_2 "Horizon color" _returnvalue)
      (`ExponentialHeightFogComponent.SetFogInscatteringColor` (`ExponentialHeightFog.Component` (`self.Fog`)) _returnvalue)
      (`MaterialInstanceDynamic.SetVectorParameterValue` _sky_material_2 "Zenith color" (`CurveLinearColor.GetClampedLinearColorValue` (`self.Zenith color curve`) (`self.Sun height`)))
      (`MaterialInstanceDynamic.SetVectorParameterValue` _sky_material_2 "Cloud color" (`CurveLinearColor.GetClampedLinearColorValue` (`self.Cloud color curve`) (`self.Sun height`)))
      (`MaterialInstanceDynamic.SetScalarParameterValue` _sky_material_2 "Horizon falloff" 3.0)
      (`MaterialInstanceDynamic.SetScalarParameterValue` _sky_material_3 "Cloud speed" (`self.Cloud speed`))
      (`MaterialInstanceDynamic.SetScalarParameterValue` _sky_material_3 "Sun brightness" (`self.Sun brightness`))
      (`MaterialInstanceDynamic.SetScalarParameterValue` _sky_material_3 "Sun height" (`KismetMathLibrary.SelectFloat` (`KismetMathLibrary.Abs` _sun_height) 0.0 (< _sun_height 0.0)))
      (`MaterialInstanceDynamic.SetScalarParameterValue` _sky_material_3 "Cloud opacity" (`self.Cloud opacity`))
      (`MaterialInstanceDynamic.SetScalarParameterValue` _sky_material_3 "Stars brightness" (`self.Stars brightness`)))))

(fn `SetTimeOfDay`
  (params (TimeOfDay :type "Float (double-precision)"))
  (bind _component (`ExponentialHeightFog.Component` (`self.Fog`)))
  (bind _lightcomponent (`Light.LightComponent` (`self.Directional light actor`)))
  (bind _output_get (set `self.TimeOfDay` TimeOfDay))
  (`|ExecutionSequence`
    (:`then_0`
      (`self.K2_SetActorRotation` (`self.Directional light actor`) (`KismetMathLibrary.MakeRotator` 0.0 (`CurveFloat.GetFloatValue` (`self.TimeOfDayCurve`) _output_get) (`self.SunYaw`)) false))
    (:`then_1`
      (`LightComponent.SetIntensity` _lightcomponent (`CurveFloat.GetFloatValue` (`self.SunIntenCurve`) _output_get))
      (`LightComponent.SetTemperature` _lightcomponent (`CurveFloat.GetFloatValue` (`self.SunTemperatureCurve`) _output_get)))
    (:`then_2`
      (`self.UpdateSunDirection`)
      (`self.RefreshMaterial`))
    (:`then_3`
      (`/Game/Landscape/Logic/GlobalLightIllum.SetIllum` (`self.GlobalIllum`) (`CurveFloat.GetFloatValue` (`self.IllumInten`) _output_get))
      (`ExponentialHeightFogComponent.SetVolumetricFogExtinctionScale` _component (`CurveFloat.GetFloatValue` (`self.Extinc`) _output_get))
      (`ExponentialHeightFogComponent.SetFogDensity` _component (`CurveFloat.GetFloatValue` (`self.FogDensity`) _output_get)))))

(fn `UpdateSunDirection`
  (bind _sky_material (`self.Sky material`))
  (bind _sun_height (`self.Sun height`))
  (bind _sky_material_2 (`self.Sky material`))
  (`MaterialInstanceDynamic.SetVectorParameterValue` _sky_material "Light direction" (`KismetMathLibrary.Conv_VectorToLinearColor` (`KismetMathLibrary.Conv_RotatorToVector` (`self.K2_GetActorRotation` (`self.Directional light actor`)))))
  (`MaterialInstanceDynamic.SetVectorParameterValue` _sky_material "Sun color" (`KismetMathLibrary.Conv_ColorToLinearColor` (`LightComponentBase.LightColor` (`Light.LightComponent` (`self.Directional light actor`)))))
  (set `self.Sun height` (`CurveFloat.GetFloatValue` (`self.TimeOfDaySunHeightCurve`) (`self.TimeOfDay`)))
  (`MaterialInstanceDynamic.SetVectorParameterValue` _sky_material_2 "Horizon color" (`CurveLinearColor.GetClampedLinearColorValue` (`self.Horizon color curve`) (`self.Sun height`)))
  (`MaterialInstanceDynamic.SetVectorParameterValue` _sky_material_2 "Zenith color" (`CurveLinearColor.GetClampedLinearColorValue` (`self.Zenith color curve`) (`self.Sun height`)))
  (`MaterialInstanceDynamic.SetVectorParameterValue` _sky_material_2 "Cloud color" (`CurveLinearColor.GetClampedLinearColorValue` (`self.Cloud color curve`) (`self.Sun height`)))
  (`MaterialInstanceDynamic.SetScalarParameterValue` _sky_material_2 "Horizon falloff" 3.0)
  (`MaterialInstanceDynamic.SetScalarParameterValue` _sky_material_2 "Sun height" (`KismetMathLibrary.SelectFloat` (`KismetMathLibrary.Abs` _sun_height) 0.0 (< _sun_height 0.0)))
  (`SkyLightComponent.SetLightColor` (`SkyLight.LightComponent` (`self.SkyLightActor`)) (`CurveLinearColor.GetClampedLinearColorValue` (`self.SkyColorCurve`) _sun_height)))

(fn `UserConstructionScript`
  (bind _returnvalue (`PrimitiveComponent.CreateDynamicMaterialInstance` (`self.SkySphereMesh`) 0 "/Game/Landscape/Logic/M_Sky_TimeOfDay_Inst.M_Sky_TimeOfDay_Inst" "None"))
  (set `self.Sky material` _returnvalue)
  (if (`self.Refresh material`)
    _
    (else
      _))
  (set `self.Refresh material` false)
  (set `self.SunYaw` (.yaw (`self.K2_GetActorRotation` (`self.Directional light actor`))))
  (`self.SetTimeOfDay` (`self.TimeOfDay`)))