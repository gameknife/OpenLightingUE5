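; Game state for OpenLight that runs a stack-based UI/game state machine and keeps lists of built-in and user camera shots.
; On clients and standalone, BeginPlay builds shots from tagged CineCameraActors, spawns collapsed UILayout data-table widgets, then pushes the first state.
; Push and pop broadcast enter/leave events, custom shots record BP_TOD time, and spawned WidgetFader actors fade widgets.
; Lumen-dependent level-streaming nodes are present but unconnected.
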(event `AddCustomShot`
  (params (Shot :type "CineCameraActor Object Reference"))
  (bind _tod (`self.GetTimeOfDay`))
  (`KismetArrayLibrary.Array_Add` (`self.UserShots`) (make `/Game/DataTables/RowStruct/BPST_OPLSingleShot` Shot (`/Game/Landscape/Logic/BP_TOD.TimeOfDay` _tod) (`KismetTextLibrary.Conv_TextToString` (`|FormatText` "用户拍摄#{0}" (`KismetArrayLibrary.Array_Length` (`self.UserShots`)))) (`KismetMathLibrary.Now`))))

(event `self.ReceiveBeginPlay`
  (bind _uilayout (`self.UILayout`))
  (`PlayerCameraManager.StartCameraFade` :`self` (`PlayerController.PlayerCameraManager` (`GameplayStatics.GetPlayerController` 0)) :`ToAlpha` 1.0 :`Duration` 0.01 :`bHoldWhenFinished` true)
  (bind _returnvalue (`|CreateWidget` "/Game/UI/Opening.Opening_C"))
  (`UserWidget.AddToViewport` _returnvalue 0)
  (if (not (and (`KismetSystemLibrary.IsServer`) (not (`KismetSystemLibrary.IsStandalone`))))
    (`|ExecutionSequence`
      (:`then_0`
        (`PlayerCameraManager.StartCameraFade` :`self` (`PlayerController.PlayerCameraManager` (`GameplayStatics.GetPlayerController` 0)) :`ToAlpha` 1.0 :`Duration` 0.01 :`bHoldWhenFinished` true))
      (:`then_1`
        (bind _outactors (`GameplayStatics.GetAllActorsOfClass` "/Script/CinematicCamera.CineCameraActor"))
        (for _array_element _outactors
          (bind _tags (`Actor.Tags` _array_element))
          (bind _returnvalue_2 (`KismetArrayLibrary.Array_Length` _tags))
          (if (> _returnvalue_2 0)
            (`KismetArrayLibrary.Array_Add` (`self.BuiltInShots`) (make `/Game/DataTables/RowStruct/BPST_OPLSingleShot` _array_element (`KismetMathLibrary.SelectFloat` (`KismetStringLibrary.Conv_StringToDouble` (`KismetStringLibrary.Conv_NameToString` (`|GetArrayItem` _tags 1))) 14.0 (> _returnvalue_2 1)) (`KismetStringLibrary.Conv_NameToString` (`|GetArrayItem` _tags)) (`KismetMathLibrary.Now`))))))
      (:`then_2`
        (bind _outrownames (`DataTableFunctionLibrary.GetDataTableRowNames` _uilayout))
        (for _array_element_2 _outrownames
          (bind _returnvalue_3 (`|GetDataTableRow` _uilayout _array_element_2)
            (:`then`
              (bind (_class _zorder _visiblestates) (break `/Game/DataTables/RowStruct/BPST_OPLUIDesc` _returnvalue_3))
              (bind _returnvalue_4 (`|CreateWidget` _class (`GameplayStatics.GetPlayerController` 0)))
              (`UserWidget.AddToViewport` _returnvalue_4 _zorder)
              (set `/Game/BluePrints/OpenLightWidgetBase.VisibleStatus` _visiblestates _returnvalue_4)
              (`Widget.SetVisibility` _returnvalue_4 "Collapsed")))))
      (:`then_3`
        (`KismetSystemLibrary.Delay` 1.0)
        (`self.PushGameState` "NewEnumerator0")
        (`PlayerCameraManager.StartCameraFade` :`self` (`PlayerController.PlayerCameraManager` (`GameplayStatics.GetPlayerController` 0)) :`FromAlpha` 1.0 :`Duration` 1.0 :`bHoldWhenFinished` true)))))

(event `PushGameState`
  (params (State :type "/Game/BluePrints/OPLGameState Enum" :default "NewEnumerator0"))
  (`KismetArrayLibrary.Array_Add` (`self.GameStateStack`) State)
  (`self.OnEnterGameState` State))

(event `PopGameState`
  (bind _returnvalue (`KismetArrayLibrary.Array_LastIndex` (`self.GameStateStack`)))
  (`self.OnLeaveGameState` (`|GetArrayItem` (`self.GameStateStack`) _returnvalue))
  (`KismetArrayLibrary.Array_Remove` (`self.GameStateStack`) _returnvalue)
  (`self.OnEnterGameState` (`|GetArrayItem` (`self.GameStateStack`) (`KismetArrayLibrary.Array_LastIndex` (`self.GameStateStack`)))))

(event `FadeInWidget`
  (params (Widget :type "/Game/BluePrints/OpenLightWidgetBase Object Reference"))
  (bind _returnvalue (`|SpawnActorFromClass` "/Game/BluePrints/WidgetFader.WidgetFader_C" (`KismetMathLibrary.MakeTransform` (0.0 0.0 0.0)) "Undefined" "OverrideRootScale" null null))
  (`/Game/BluePrints/WidgetFader.FadeWidget` _returnvalue Widget true))

(event `FadeOutWidget`
  (params (Widget :type "/Game/BluePrints/OpenLightWidgetBase Object Reference"))
  (bind _returnvalue (`|SpawnActorFromClass` "/Game/BluePrints/WidgetFader.WidgetFader_C" (`KismetMathLibrary.MakeTransform` (0.0 0.0 0.0)) "Undefined" "OverrideRootScale" null null))
  (`/Game/BluePrints/WidgetFader.FadeWidget` _returnvalue Widget false))

(fn `GetTimeOfDay`
  (returns (TOD :type "/Game/Landscape/Logic/BP_TOD Object Reference"))
  (`/Engine/EditorBlueprintResources/StandardMacros.IsValid` (`self.TOD`)
    (:`Is Valid`
      _)
    (:`Is Not Valid`
      (bind _returnvalue (`GameplayStatics.GetActorOfClass` "/Game/Landscape/Logic/BP_TOD.BP_TOD_C"))
      (set `self.TOD` _returnvalue)))
  (return (`self.TOD`)))

(fn `GetTimeOfDayDigitName`
  (returns (OutName :type Text))
  (bind _tod (`self.GetTimeOfDay`))
  (`/Engine/EditorBlueprintResources/StandardMacros.IsValid` _tod
    (:`Is Valid`
      (bind _returnvalue (+ (`/Game/Landscape/Logic/BP_TOD.TimeOfDay` _tod) 0.001))
      (return (`|FormatText` "{0}:{1}" (`KismetTextLibrary.Conv_IntToText` (`KismetMathLibrary.FFloor` _returnvalue) false true 2) (`KismetTextLibrary.Conv_IntToText` (`KismetMathLibrary.FFloor` (* (`KismetMathLibrary.Fraction` _returnvalue) 60.0)) false true 2))))
    (:`Is Not Valid`
      (return "00:00"))))

(fn `GetTopState`
  (returns (State :type "/Game/BluePrints/OPLGameState Enum"))
  (bind _gamestatestack (`self.GameStateStack`))
  (return (`|GetArrayItem` _gamestatestack (`KismetArrayLibrary.Array_LastIndex` _gamestatestack))))

(fn `UserConstructionScript`)