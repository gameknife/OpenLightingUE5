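; Player controller for a photography mode that switches possession between the main pawn and a spawned drone character with a view blend.
; It spawns a cine camera with lens cycling and aperture adjustment, shown while QuickShot is held through debounced view switches and fades.
; TakeShot saves a duplicate camera actor as a custom shot in the OPL game state.
; That game state's stack tracks camera and gallery modes and relays camera events.
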(event `self.ReceiveBeginPlay`
  (bind _output_get (set `self.MainPawn` (`GameplayStatics.GetPlayerCharacter` 0)))
  (bind _returnvalue (`|SpawnActorFromClass` "/Game/ThirdPersonBP/Blueprints/ThirdPersonCharacter.ThirdPersonCharacter_C" (`self.GetTransform` _output_get) "AdjustIfPossibleButAlwaysSpawn" "OverrideRootScale" null null))
  (set `self.DronePawn` _returnvalue)
  (set `self.bShowMouseCursor` true)
  (`self.InitCineCamera`))

(event `InputAction|SwitchCharacter`
  (params (Key :type "Key Structure"))
  (bind _returnvalue (`GameplayStatics.GetPlayerController` 0))
  (bind _mainpawn (`self.MainPawn`))
  (bind _dronepawn (`self.DronePawn`))
  (:`Pressed`
    (if (== (`GameplayStatics.GetPlayerCharacter` 0) (`self.MainPawn`))
      (`self.UnPossess` _returnvalue)
      (`self.Possess` _returnvalue _dronepawn)
      (`self.SetViewTargetWithBlend` (`self.MainPawn`))
      (`self.SetViewTargetWithBlend` _dronepawn 0.5)
      (else
        (`self.UnPossess` _returnvalue)
        (`self.Possess` _returnvalue _mainpawn)
        (`self.SetViewTargetWithBlend` (`self.DronePawn`))
        (`self.SetViewTargetWithBlend` _mainpawn 0.5)))))

(event `InitCineCamera`
  (bind _returnvalue (`CineCameraActor.GetCineCameraComponent` (`self.CineCamera`)))
  (bind _returnvalue_2 (`|SpawnActorFromClass` "/Script/CinematicCamera.CineCameraActor" (`self.GetTransform`) "Undefined" "OverrideRootScale" null null))
  (set `self.CineCamera` _returnvalue_2)
  (`CineCameraComponent.SetFilmbackPresetByName` _returnvalue "Full Frame DSLR")
  (`CineCameraComponent.SetLensPresetByName` _returnvalue "30mm Prime f/1.4")
  (set `CineCameraComponent.CurrentAperture` 1.4 _returnvalue)
  (set `CineCameraComponent.FocusSettings` (make `CameraFocusSettings` "Manual" 500.0) _returnvalue)
  (bind _returnvalue_3 (`CineCameraComponent.GetLensPresetsCopy`))
  (for _array_element _returnvalue_3
    (`KismetArrayLibrary.Array_Add` (`self.LensPresets`) (`.Name` (break `NamedLensPreset` _array_element)))))

(event `TakeShot`
  (bind _cinecamera (`self.CineCamera`))
  (bind _returnvalue (`CineCameraActor.GetCineCameraComponent` _cinecamera))
  (bind _returnvalue_2 (`|SpawnActorFromClass` "/Script/CinematicCamera.CineCameraActor" (`self.GetTransform` _cinecamera) "Undefined" "OverrideRootScale" null null))
  (bind _returnvalue_3 (`CineCameraActor.GetCineCameraComponent` _returnvalue_2))
  (`CineCameraComponent.SetLensPresetByName` _returnvalue_3 (`CineCameraComponent.GetLensPresetName` _returnvalue))
  (`CineCameraComponent.SetFilmbackPresetByName` _returnvalue_3 (`CineCameraComponent.GetFilmbackPresetName` _returnvalue))
  (set `CineCameraComponent.CurrentAperture` (`CineCameraComponent.CurrentAperture` _returnvalue) _returnvalue_3)
  (set `CineCameraComponent.FocusSettings` (`CineCameraComponent.FocusSettings` _returnvalue) _returnvalue_3)
  (bind _gs (`/Game/BluePrints/GlobalBFL.GetOPLGameState` self))
  (`/Game/BluePrints/OpenLightGameState.AddCustomShot` _gs _returnvalue_2)
  (`/Game/BluePrints/OpenLightGameState.OnDoCameraAction` _gs "NewEnumerator4" true 0.0))

(event `SwitchCamera`
  (params (Cine :type Boolean))
  (bind _playercameramanager (`PlayerController.PlayerCameraManager` (`GameplayStatics.GetPlayerController` 0)))
  (bind _gs (`/Game/BluePrints/GlobalBFL.GetOPLGameState` self))
  (bind _state (`/Game/BluePrints/OpenLightGameState.GetTopState` _gs))
  (if (!= (`|EnumEquality` _state "NewEnumerator1") Cine)
    (if (> (- (`GameplayStatics.GetTimeSeconds`) (`self.LastChangeCamTime`)) 0.5)
      (set `self.LastChangeCamTime` (`GameplayStatics.GetTimeSeconds`))
      (`|ExecutionSequence`
        (:`then_0`
          (`self.SetViewTargetWithBlend` (`GameplayStatics.GetPlayerController` 0) (select `bool` Cine :`false` self :`true` (`self.CineCamera`) :!type "Actor Object Reference") 0.25 "VTBlend_Linear" 0.0 false))
        (:`then_1`
          (if Cine
            (`PlayerCameraManager.StartCameraFade` :`self` _playercameramanager :`ToAlpha` 1.0 :`Duration` 0.35 :`bHoldWhenFinished` true)
            (`KismetSystemLibrary.Delay` 0.5)
            (if Cine
              _
              (else
                _))
            (`PlayerCameraManager.StartCameraFade` :`self` _playercameramanager :`FromAlpha` 1.0 :`Duration` 0.2 :`bHoldWhenFinished` true)
            (bind _gs_2 (`/Game/BluePrints/GlobalBFL.GetOPLGameState` (`GameplayStatics.GetPlayerController` 0)))
            (`/Game/BluePrints/OpenLightGameState.OnChangeCineCamera` _gs_2 (select `bool` Cine :`true` (`self.CineCamera`)))))
        (:`then_2`
          (bind _gs_3 (`/Game/BluePrints/GlobalBFL.GetOPLGameState` self))
          (if Cine
            (`/Game/BluePrints/OpenLightGameState.PushGameState` _gs_3 "NewEnumerator1")
            (else
              (`/Game/BluePrints/OpenLightGameState.PopGameState` _gs_3))))))))

(event `NextLens`
  (bind _playercameramanager (`PlayerController.PlayerCameraManager` (`GameplayStatics.GetPlayerController` 0)))
  (bind _output_get (set `self.LensPresetsCurIdx` (mod (+ (`self.LensPresetsCurIdx`) 1) (`KismetArrayLibrary.Array_Length` (`self.LensPresets`)))))
  (bind _output (`|GetArrayItem` (`self.LensPresets`) _output_get))
  (`CineCameraComponent.SetLensPresetByName` (`CineCameraActor.GetCineCameraComponent` (`self.CineCamera`)) _output)
  (bind _gs (`/Game/BluePrints/GlobalBFL.GetOPLGameState` (`GameplayStatics.GetPlayerController` 0)))
  (`/Game/BluePrints/OpenLightGameState.OnShowTips` _gs _output 1.0)
  (`/Game/BluePrints/OpenLightGameState.OnChangeCineCamera` _gs (`self.CineCamera`))
  (`/Game/BluePrints/OpenLightGameState.OnDoCameraAction` _gs "NewEnumerator1" true 0.0)
  (`PlayerCameraManager.StartCameraFade` :`self` _playercameramanager :`ToAlpha` 1.0 :`Duration` 0.1 :`bHoldWhenFinished` true)
  (`KismetSystemLibrary.Delay` 0.15)
  (`PlayerCameraManager.StartCameraFade` :`self` _playercameramanager :`FromAlpha` 1.0 :`Duration` 0.1 :`bHoldWhenFinished` true))

(event `DecreaseAperture`
  (bind _returnvalue (`CineCameraActor.GetCineCameraComponent` (`self.CineCamera`)))
  (set `CineCameraComponent.CurrentAperture` (- (`CineCameraComponent.CurrentAperture` _returnvalue) 0.1) _returnvalue)
  (bind _gs (`/Game/BluePrints/GlobalBFL.GetOPLGameState` self :!label _label))
  (`/Game/BluePrints/OpenLightGameState.OnDoCameraAction` _gs "NewEnumerator2" true 0.0))

(event `IncreaseAperture`
  (bind _returnvalue (`CineCameraActor.GetCineCameraComponent` (`self.CineCamera`)))
  (set `CineCameraComponent.CurrentAperture` (+ (`CineCameraComponent.CurrentAperture` _returnvalue) 0.1) _returnvalue)
  (goto _label))

(event `InputAction|ChangeLens`
  (params (Key :type "Key Structure"))
  (:`Pressed`
    (`self.NextLens`)))

(event `InputAction|QuickGallery`
  (params (Key :type "Key Structure"))
  (:`Pressed`
    (bind _gs (`/Game/BluePrints/GlobalBFL.GetOPLGameState` self))
    (`/Game/BluePrints/OpenLightGameState.PushGameState` _gs "NewEnumerator3"))
  (:`Released`
    (bind _gs_2 (`/Game/BluePrints/GlobalBFL.GetOPLGameState` self))
    (bind _state (`/Game/BluePrints/OpenLightGameState.GetTopState` _gs_2))
    (if (`|EnumEquality` _state "NewEnumerator3")
      (`/Game/BluePrints/OpenLightGameState.PopGameState` _gs_2))))

(event `InputAction|QuickShot`
  (params (Key :type "Key Structure"))
  (:`Pressed`
    (`self.SwitchCamera` true))
  (:`Released`
    (`self.SwitchCamera` false)))

(event `InputAction|TakeShot`
  (params (Key :type "Key Structure"))
  (:`Pressed`
    (bind _gs (`/Game/BluePrints/GlobalBFL.GetOPLGameState` self))
    (bind _state (`/Game/BluePrints/OpenLightGameState.GetTopState` _gs))
    (if (`|EnumEquality` _state "NewEnumerator1")
      (`self.TakeShot`))))

(event `InputAction|IncreaseAperture`
  (params (Key :type "Key Structure"))
  (:`Pressed`
    (`self.IncreaseAperture`)))

(event `InputAction|DecreaseAperture`
  (params (Key :type "Key Structure"))
  (:`Pressed`
    (`self.DecreaseAperture`)))

(fn `UserConstructionScript`)